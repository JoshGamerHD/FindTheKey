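; Game mode Blueprint that spawns local players at level start and keeps a running TargetScore.
; On BeginPlay it caches all PlayerStart actors, then for each index up to MaxPlayerCount finds starts whose tag matches that index.
; Each match creates a player, spawns a BP_Character there, applies the Character2Colour material, possesses it and records it in Players.
; AddScore adds the given amount to TargetScore.
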(event `self.ReceiveBeginPlay`
  (`self.GetPlayerStart`)
  (`self.spawnPlayer`))

(event `AddScore`
  (params (Addscore :type Integer))
  (set `self.TargetScore` (+ Addscore (`self.TargetScore`))))

(fn `GetPlayerStart`
  (bind _outactors (`GameplayStatics.GetAllActorsOfClass` "/Script/Engine.PlayerStart"))
  (set `self.PlayerStartArray` _outactors))

(fn `spawnPlayer`
  (for _index (range (`self.MaxPlayerCount`))
    (set `self.Index` _index)
    (for _array_element (`self.PlayerStartArray`)
      (if (== (`PlayerStart.PlayerStartTag` _array_element) (`KismetStringLibrary.Conv_StringToName` (`KismetStringLibrary.Conv_IntToString` (`self.Index`))))
        (`GameplayStatics.CreatePlayer` (`self.Index`))
        (bind _returnvalue (`|SpawnActorFromClass` "/Game/Blueprints/BP_Character.BP_Character_C" (`self.GetTransform` _array_element) "AlwaysSpawn" "OverrideRootScale" null null))
        (`PrimitiveComponent.SetMaterial` (`Character.Mesh` _returnvalue) 0 "/Game/Assets/Materials/Character2Colour.Character2Colour")
        (`Controller.Possess` (`GameplayStatics.GetPlayerController` (`self.Index`)) _returnvalue)
        (`KismetArrayLibrary.Array_AddUnique` (`self.Players`) _returnvalue)))))

(fn `UserConstructionScript`)