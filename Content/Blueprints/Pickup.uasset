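; Collectible pickup actor that awards score when the player character enters its Box trigger.
; On overlap with BP_Character it spawns an explosion at the Cube, destroys itself, adds Score through BP_Gamemode and plays a sound.
; An unfiltered end-overlap from any actor starts a delayed self-destruct with a debug "no point" message.
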(event `self.Box.OnComponentBeginOverlap`
  (params (OverlappedComponent :type "PrimitiveComponent Object Reference") (OtherActor :type "Actor Object Reference") (OtherComp :type "PrimitiveComponent Object Reference") (OtherBodyIndex :type Integer) (bFromSweep :type Boolean) (SweepResult :type "HitResult Structure (by ref)"))
  (bind _cube (`self.Cube`))
  (cast `/Game/Blueprints/BP_Character` OtherActor)
  (`GameplayStatics.SpawnEmitterAtLocation` "/Game/StarterContent/Particles/P_Explosion.P_Explosion" (`SceneComponent.K2_GetComponentLocation` _cube) (`SceneComponent.K2_GetComponentRotation` _cube))
  (`self.K2_DestroyActor`)
  (`KismetSystemLibrary.PrintString` "yes")
  (bind _asbp_gamemode (cast `/Game/Blueprints/BP_Gamemode` (`GameplayStatics.GetGameMode`)))
  (`/Game/Blueprints/BP_Gamemode.AddScore` _asbp_gamemode (`self.Score`))
  (`GameplayStatics.PlaySound2D` "/Game/StarterContent/Audio/Explosion01.Explosion01" 0.5 1.0 0.0 null null))

(event `self.Box.OnComponentEndOverlap`
  (params (OverlappedComponent :type "PrimitiveComponent Object Reference") (OtherActor :type "Actor Object Reference") (OtherComp :type "PrimitiveComponent Object Reference") (OtherBodyIndex :type Integer))
  (`KismetSystemLibrary.Delay` 6.0)
  (`self.K2_DestroyActor`)
  (`KismetSystemLibrary.PrintString` "no point for you"))

(fn `UserConstructionScript`)