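; Shared multiplayer camera that frames up to four players taken from BP_Gamemode and becomes the player controllers' view target.
; A looping 0.001-second timer sets spring arm length to the largest distance between any two players, clamped to min and max.
; It also interpolates the actor toward the players' average location, with missing players adding zero.
; SetCameraRotation averages player facing similarly but is never called here.
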(event `self.ReceiveBeginPlay`
  (`KismetSystemLibrary.Delay` 0.001)
  (`self.ClassSetup`)
  (`KismetSystemLibrary.K2_SetTimer` null "UpdateCamera" 0.001 true))

(event `UpdateCamera`
  (`self.SetArmLength`)
  (`self.SetCameraPos`))

(fn `Calc Distance`
  (params (PlayerRef1 :type "/Game/Blueprints/BP_Character Object Reference") (PlayerRef2 :type "/Game/Blueprints/BP_Character Object Reference"))
  (returns (LocalDistance1 :type "Float (double-precision)"))
  (locals (LocalDistance :type "Float (double-precision)" :default 0.0))
  ;[0.2624 0.1136 1] Checks For Local Distance between each character then does a branch to see if it is valid or not and if it is then it will set the distance between the different reference players
  (if (and (`KismetSystemLibrary.IsValid` PlayerRef1) (`KismetSystemLibrary.IsValid` PlayerRef2))
    (set `local.LocalDistance` (`self.GetDistanceTo` PlayerRef1 PlayerRef2))
    (else
      (set `local.LocalDistance` 0.0)))
  (return (`local.LocalDistance`)))

(fn `ClassSetup`
  (bind _asbp_gamemode (cast `/Game/Blueprints/BP_Gamemode` (`GameplayStatics.GetGameMode`)))
  (bind _output_get (set `self.BP_Gamemode` _asbp_gamemode))
  (set `self.PlayerREF` (`/Game/Blueprints/BP_Gamemode.Players` _output_get))
  (bind _outactors (`GameplayStatics.GetAllActorsOfClass` "/Script/Engine.PlayerController"))
  (`PlayerController.SetViewTargetWithBlend` _outactors self 0.0 "VTBlend_Linear" 0.0 false)
  (for (_array_element _array_index) (`self.PlayerREF`)
    (switch `int` _array_index
      (:`0`
        (set `self.P1` _array_element))
      (:`1`
        (set `self.P2` _array_element))
      (:`2`
        (set `self.P3` _array_element))
      (:`3`
        (set `self.P4` _array_element)))))

(fn `GetLocation`
  (params (Player :type "/Game/Blueprints/BP_Character Object Reference"))
  (returns (PlayerLocation :type "Vector Structure"))
  (locals (LocalLocation :type "Vector Structure" :default (0.0 0.0 0.0)) (LocationRotation :type Boolean))
  (`/Engine/EditorBlueprintResources/StandardMacros.IsValid` Player
    (:`Is Valid`
      (set `local.LocalLocation` (`self.K2_GetActorLocation` Player)))
    (:`Is Not Valid`
      (set `local.LocalLocation` (0.0 0.0 0.0))))
  (return (`local.LocalLocation`)))

(fn `GetRotation`
  (params (Player :type "/Game/Blueprints/BP_Character Object Reference"))
  (returns (PlayerRotation :type "Rotator Structure"))
  (locals (LocalLocation :type "Vector Structure" :default (0.0 0.0 0.0)) (LocationRotation :type "Rotator Structure"))
  (`/Engine/EditorBlueprintResources/StandardMacros.IsValid` Player
    (:`Is Valid`
      (set `local.LocationRotation` (`self.K2_GetActorRotation` Player)))
    (:`Is Not Valid`
      (set `local.LocationRotation` (struct))))
  (return (`local.LocationRotation`)))

(fn `SetArmLength`
  (bind _p1 (`self.P1`))
  (bind _p2 (`self.P2`))
  (bind _p3 (`self.P3`))
  (bind _p4 (`self.P4`))
  (set `SpringArmComponent.TargetArmLength` (`KismetMathLibrary.FClamp` (`.MaxValue` (`KismetMathLibrary.MaxOfFloatArray` (`|MakeArray` (`self.Calc Distance` _p1 _p2) (`self.Calc Distance` _p1 _p3) (`self.Calc Distance` _p1 _p4) (`self.Calc Distance` _p2 _p3) (`self.Calc Distance` _p2 _p4) (`self.Calc Distance` _p3 _p4)))) (`self.MinArmLength`) (`self.MaxArmLength`)) (`self.SpringArm`)))

(fn `SetCameraPos`
  (set `self.TargetPos` (/ (+ (`self.GetLocation` (`self.P1`)) (`self.GetLocation` (`self.P2`)) (`self.GetLocation` (`self.P3`)) (`self.GetLocation` (`self.P4`))) (`KismetMathLibrary.Conv_IntToDouble` (`KismetArrayLibrary.Array_Length` (`self.PlayerREF`)))))
  (`self.K2_SetActorLocation` (`KismetMathLibrary.VInterpTo` (`self.PreviousPos`) (`self.TargetPos`) (`GameplayStatics.GetWorldDeltaSeconds`) (`self.InterpSpeed`)))
  (set `self.PreviousPos` (`self.K2_GetActorLocation`)))

(fn `SetCameraRotation`
  (set `self.TargetPos` (/ (+ (`KismetMathLibrary.Conv_RotatorToVector` (`self.GetRotation` (`self.P1`))) (`KismetMathLibrary.Conv_RotatorToVector` (`self.GetRotation` (`self.P2`))) (`KismetMathLibrary.Conv_RotatorToVector` (`self.GetRotation` (`self.P3`))) (`KismetMathLibrary.Conv_RotatorToVector` (`self.GetRotation` (`self.P4`)))) (`KismetMathLibrary.Conv_IntToDouble` (`KismetArrayLibrary.Array_Length` (`self.PlayerREF`)))))
  (`self.K2_SetActorRotation` (`KismetMathLibrary.Conv_VectorToRotator` (`KismetMathLibrary.VInterpTo` (`self.PreviousPos`) (`self.TargetPos`) (`GameplayStatics.GetWorldDeltaSeconds`) (`self.InterpSpeed`))))
  (set `self.PreviousPos` (`KismetMathLibrary.Conv_RotatorToVector` (`self.K2_GetActorRotation`))))

(fn `UserConstructionScript`)